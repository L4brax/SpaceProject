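; BP_EnemySpline is an actor that moves an enemy ship component, Ship0, along its spline.
; Each Tick advances a distance counter by SplineSpeed times delta time, then samples the spline's location and rotation there, keeping the ship's scale.
; The world-space sample is applied as Ship0's relative transform, and the distance is never wrapped or reset.
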(event `self.ReceiveTick`
  (params (DeltaSeconds :type "Float (single-precision)"))
  (bind _returnvalue (`SplineComponent.GetTransformAtDistanceAlongSpline` (`self.Spline`) (`self.DistanceAlongSpline`) "World" false))
  (set `self.DistanceAlongSpline` (+ (* DeltaSeconds (`self.SplineSpeed`)) (`self.DistanceAlongSpline`)))
  (`SceneComponent.K2_SetRelativeTransform` (`self.Ship_0`) (`KismetMathLibrary.MakeTransform` (.location _returnvalue) (`KismetMathLibrary.MakeRotator` (.roll (.rotation _returnvalue)) (.pitch (.rotation _returnvalue)) (.yaw (.rotation _returnvalue))) (`SceneComponent.RelativeScale3D` (`self.Ship_0`))) false false))

(fn `UserConstructionScript`)