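; Player-controlled spaceship Blueprint that flies with six-axis-style steering through Enhanced Input actions.
; Accelerate input accumulates forward speed, while Move and Roll inputs interpolate yaw, pitch and roll speeds toward scaled turn targets.
; Tick applies those speeds as a swept local forward offset and local rotation, scaled by delta time.
; Debug prints remain, and the IMC_Space mapping context setup is disconnected, so it never runs here.
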(event `self.ReceiveBeginPlay`)

(event `self.ReceiveTick`
  (params (DeltaSeconds :type "Float (single-precision)"))
  (bind _returnvalue (`GameplayStatics.GetWorldDeltaSeconds`))
  (`self.K2_AddActorLocalOffset` (`KismetMathLibrary.MakeVector` (* DeltaSeconds (`self.CurrentForwardSpeed`))) true)
  (`self.K2_AddActorLocalRotation` (`KismetMathLibrary.MakeRotator` (* _returnvalue (`self.CurrentRollSpeed`)) (* (`self.CurrentPitchSpeed`) _returnvalue) (* _returnvalue (`self.CurrentYawSpeed`)))))

(event `EnhancedInput|/Game/Input/IA_Accelerate`
  (params (ActionValue :type "Float (double-precision)") (ElapsedSeconds :type "Float (double-precision)") (TriggeredSeconds :type "Float (double-precision)") (InputAction :type "InputAction Object Reference" :default "/Game/Input/IA_Accelerate.IA_Accelerate"))
  (bind _acceleration (`self.Acceleration`))
  (:`Triggered`
    (bind _output_get (set `self.CurrentForwardSpeed` (+ (* (`KismetMathLibrary.SelectFloat` (* ActionValue _acceleration) (* _acceleration 0.5) (!= ActionValue 0.0)) (`GameplayStatics.GetWorldDeltaSeconds`)) (`self.CurrentForwardSpeed`))))
    (`KismetSystemLibrary.PrintString` (`KismetStringLibrary.Conv_DoubleToString` _output_get))))

(event `EnhancedInput|/Game/Input/IA_Move`
  (params (ActionValue :type "Vector2D Structure") (ElapsedSeconds :type "Float (double-precision)") (TriggeredSeconds :type "Float (double-precision)") (InputAction :type "InputAction Object Reference" :default "/Game/Input/IA_Move.IA_Move"))
  (bind (_x _y) (`KismetMathLibrary.BreakVector2D` ActionValue))
  (:`Triggered`
    (set `self.CurrentYawSpeed` (`KismetMathLibrary.FInterpTo` (`self.CurrentYawSpeed`) (* (`self.TurnSpeed`) _x) (`GameplayStatics.GetWorldDeltaSeconds`) 2.0))
    (set `self.CurrentPitchSpeed` (`KismetMathLibrary.FInterpTo` (`self.CurrentPitchSpeed`) (* (`self.TurnSpeed`) _y -1.0) (`GameplayStatics.GetWorldDeltaSeconds`) 2.0))))

(event `EnhancedInput|/Game/Input/IA_Roll`
  (params (ActionValue :type "Float (double-precision)") (ElapsedSeconds :type "Float (double-precision)") (TriggeredSeconds :type "Float (double-precision)") (InputAction :type "InputAction Object Reference" :default "/Game/Input/IA_Roll.IA_Roll"))
  (:`Triggered`
    (set `self.CurrentRollSpeed` (`KismetMathLibrary.FInterpTo` (`self.CurrentRollSpeed`) (* (`self.TurnSpeed`) ActionValue) (`GameplayStatics.GetWorldDeltaSeconds`) 2.0)))
  (:`Completed`
    (set `self.CurrentRollSpeed` (`KismetMathLibrary.FInterpTo` (`self.CurrentRollSpeed`) 0.0 (`GameplayStatics.GetWorldDeltaSeconds`)))
    (`KismetSystemLibrary.PrintString` "Hello")))

(fn `UserConstructionScript`)